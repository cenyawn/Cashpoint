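; Core objective that runs a two-team zone-control match, handling scoring, win check, reset and HUD updates.
; A timer counts living team pawns in a box, weighting each team's count by its owned facilities.
; After an unlock delay, each cycle pays a point to the previously locked owner, then locks the stronger side until a team reaches WinScore.
; HUD pushes mostly fire only on changed values; the enemy respawn loop on reset is unconnected.
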(event `self.ReceiveBeginPlay`
  (`KismetSystemLibrary.K2_SetTimerDelegate` (delegate `UpdateCountsTick`) 0.2 true)
  (set `self.PrevOwner` 2))

(event `self.ReceiveTick`
  (params (DeltaSeconds :type "Float (single-precision)"))
  (if (not (`self.bEnded`))
    (`self.UpdateMatch` DeltaSeconds)))

(event `UpdateCountsTick`
  (`self.UpdateCounts`))

(fn `ComputeEffective`
  (set `self.MultA` (+ 1.0 (* (`KismetMathLibrary.Conv_IntToDouble` (`self.OwnedCountA`)) 0.25)))
  (set `self.EffA` (* (`KismetMathLibrary.Conv_IntToDouble` (`self.CountA`)) (`self.MultA`)))
  (set `self.MultB` (+ 1.0 (* (`KismetMathLibrary.Conv_IntToDouble` (`self.OwnedCountB`)) 0.25)))
  (set `self.EffB` (* (`KismetMathLibrary.Conv_IntToDouble` (`self.CountB`)) (`self.MultB`))))

(fn `LockOwner`
  (bind _effa (`self.EffA`))
  (bind _effb (`self.EffB`))
  (if (> _effa _effb)
    (set `self.PrevOwner` 0)
    (elif (> _effb _effa)
      (set `self.PrevOwner` 1)
      (else
        (set `self.PrevOwner` 2)))))

(fn `OnFacilityOwnerChanged`
  (params (FacilityId :type Name) (Team :type Integer))
  (`self.RefreshFacilities`))

(fn `PayScore`
  (params (Owner :type Integer))
  (if (== Owner 0)
    (set `self.ScoreA` (+ (`self.ScoreA`) 1))
    (elif (== Owner 1)
      (set `self.ScoreB` (+ (`self.ScoreB`) 1)))))

(fn `PushHUD`
  (params (bForce :type Boolean))
  (bind _hudwidget (`self.HUDWidget`))
  (bind _scorea (`self.ScoreA`))
  (bind _prevowner (`self.PrevOwner`))
  (bind _matchtime (`self.MatchTime`))
  (bind _scoreb (`self.ScoreB`))
  (bind _bcoreunlocked (`self.bCoreUnlocked`))
  (bind _counta (`self.CountA`))
  (bind _countb (`self.CountB`))
  (bind _effa (`self.EffA`))
  (bind _effb (`self.EffB`))
  (bind _returnvalue (`KismetMathLibrary.FFloor` _matchtime))
  (bind _returnvalue_2 (`KismetMathLibrary.Round` (* (`self.MultA`) 100.0)))
  (bind _returnvalue_3 (`KismetMathLibrary.SelectInt` -1 (`KismetMathLibrary.FCeil` (- (`self.CoreUnlockDelay`) _matchtime)) _bcoreunlocked))
  (if (`KismetSystemLibrary.IsValid` _hudwidget)
    (`|ExecutionSequence`
      (:`then_0`
        (if (or bForce (or (!= _scorea (`self.LastScoreA`)) (!= _scoreb (`self.LastScoreB`))))
          (`/Game/CODE/UI/UI_ZoneHUD.SetZoneScore` _hudwidget _scorea _scoreb)
          (set `self.LastScoreA` _scorea)
          (set `self.LastScoreB` _scoreb)))
      (:`then_1`
        (if (or bForce (or (or (or (!= _counta (`self.LastCountA`)) (!= _countb (`self.LastCountB`))) (!= _effa (`self.LastEffA`))) (!= _effb (`self.LastEffB`))))
          (`/Game/CODE/UI/UI_ZoneHUD.SetZoneCounts` _hudwidget _counta _countb _effa _effb)
          (`/Game/CODE/UI/UI_ZoneHUD.SetZoneCountsBoth` _hudwidget _counta _countb)
          (set `self.LastCountA` _counta)
          (set `self.LastCountB` _countb)
          (set `self.LastEffA` _effa)
          (set `self.LastEffB` _effb)))
      (:`then_2`
        (if (or bForce (!= _prevowner (`self.LastOwner`)))
          (`/Game/CODE/UI/UI_ZoneHUD.SetZoneOwner` _hudwidget _prevowner)
          (`/Game/CODE/UI/UI_ZoneHUD.SetCycleOwnerText` _hudwidget _prevowner)
          (set `self.LastOwner` _prevowner)))
      (:`then_3`
        (`/Game/CODE/UI/UI_ZoneHUD.SetCycleProgress` _hudwidget (/ (`self.CycleTimer`) (`self.CyclePeriod`))))
      (:`then_4`
        (if (or bForce (!= _returnvalue (`self.LastTimerSecond`)))
          (`/Game/CODE/UI/UI_ZoneHUD.SetMatchTime` (`self.HUDWidget`) _returnvalue)
          (set `self.LastTimerSecond` _returnvalue)))
      (:`then_5`
        (if (or bForce (!= _returnvalue_2 (`self.LastMultPercent`)))
          (`/Game/CODE/UI/UI_ZoneHUD.SetMultiplierPercentText` _hudwidget _returnvalue_2)
          (set `self.LastMultPercent` _returnvalue_2)))
      (:`then_6`
        (if (or bForce (!= _returnvalue_3 (`self.LastUnlockSecond`)))
          (`/Game/CODE/UI/UI_ZoneHUD.SetCoreUnlockText` _hudwidget _returnvalue_3 _bcoreunlocked)
          (set `self.LastUnlockSecond` _returnvalue_3))))))

(fn `RefreshFacilities`
  (bind _hudwidget (`self.HUDWidget`))
  (set `self.OwnedCountA` 0)
  (set `self.OwnedCountB` 0)
  (for _array_element (`self.Facilities`)
    (if (`KismetSystemLibrary.IsValid` _array_element)
      (if (== (`/Game/CODE/Objective/BP_Facility.State` _array_element) 3)
        (bind _ownerteam (`/Game/CODE/Objective/BP_Facility.OwnerTeam` _array_element))
        (if (== _ownerteam 0)
          (set `self.OwnedCountA` (+ (`self.OwnedCountA`) 1))
          (elif (== _ownerteam 1)
            (set `self.OwnedCountB` (+ (`self.OwnedCountB`) 1)))))))
  (`self.ComputeEffective`)
  (if (`KismetSystemLibrary.IsValid` _hudwidget)
    (`/Game/CODE/UI/UI_ZoneHUD.SetFacilityStars` _hudwidget (`self.OwnedCountA`) (`self.OwnedCountB`))))

(fn `RegisterFacility`
  (params (Facility :type "/Game/CODE/Objective/BP_Facility Object Reference"))
  (bind _facilities (`self.Facilities`))
  (if (not (`KismetArrayLibrary.Array_Contains` _facilities Facility))
    (`KismetArrayLibrary.Array_Add` _facilities Facility))
  (`self.RefreshFacilities`))

(fn `ResetMatch`
  (bind _hudwidget (`self.HUDWidget`))
  (set `self.MatchTime` 0.0)
  (set `self.CycleTimer` 0.0)
  (set `self.CycleIndex` 0)
  (set `self.bEnded` false)
  (set `self.WinnerTeam` 2)
  (set `self.PrevOwner` 2)
  (set `self.ScoreA` 0)
  (set `self.ScoreB` 0)
  (set `self.OwnedCountA` 0)
  (set `self.OwnedCountB` 0)
  (set `self.LastScoreA` -1)
  (set `self.LastScoreB` -1)
  (set `self.LastOwner` -1)
  (set `self.LastCountA` -1)
  (set `self.LastCountB` -1)
  (set `self.LastEffA` -1.0)
  (set `self.LastEffB` -1.0)
  (set `self.LastCycleIndex` -1)
  (`self.PushHUD` true)
  (for _array_element (`self.Facilities`)
    (if (`KismetSystemLibrary.IsValid` _array_element)
      (`/Game/CODE/Objective/BP_Facility.ResetFacility` _array_element)))
  (`self.RefreshFacilities`)
  (set `self.LastTimerSecond` -1)
  (`self.OnMatchReset`)
  (`self.UpdateCounts`)
  (set `self.bCoreUnlocked` false)
  (set `self.LastUnlockSecond` -1)
  (set `self.LastMultPercent` -1)
  (`|ExecutionSequence`
    (:`then_0`
      (if (`KismetSystemLibrary.IsValid` _hudwidget)
        (`/Game/CODE/UI/UI_ZoneHUD.HideResultText` _hudwidget)))
    (:`then_1`
      (bind _outactors (`GameplayStatics.GetAllActorsOfClass` "/Game/CODE/AI/BP_EnemyAI.BP_EnemyAI_C")))))

(fn `SetHUD`
  (params (Widget :type "/Game/CODE/UI/UI_ZoneHUD Object Reference"))
  (bind _hudwidget (`self.HUDWidget`))
  (set `self.HUDWidget` Widget)
  (`self.PushHUD` true)
  (if (`KismetSystemLibrary.IsValid` _hudwidget)
    (`/Game/CODE/UI/UI_ZoneHUD.SetFacilityStars` _hudwidget (`self.OwnedCountA`) (`self.OwnedCountB`))))

(fn `UpdateCounts`
  (set `self.CountA` 0)
  (set `self.CountB` 0)
  (bind _outactors (`KismetSystemLibrary.BoxOverlapActors` (`self.K2_GetActorLocation`) (`self.BoxExtent`) (`|MakeArray` (enumliteral `EObjectTypeQuery` "ObjectTypeQuery3"))))
  (for _array_element _outactors
    (bind _returnvalue (`self.GetComponentByClass` _array_element "/Game/CODE/Combat/BP_HealthComponent.BP_HealthComponent_C"))
    (if (`KismetSystemLibrary.IsValid` _returnvalue)
      (bind _asbp_health_component (cast `/Game/CODE/Combat/BP_HealthComponent` _returnvalue))
      (if (not (`/Game/CODE/Combat/BP_HealthComponent.bDead` _asbp_health_component))
        (bind _teamid (`/Game/CODE/Combat/BP_HealthComponent.TeamId` _asbp_health_component))
        (if (== _teamid 0)
          (set `self.CountA` (+ (`self.CountA`) 1))
          (elif (== _teamid 1)
            (set `self.CountB` (+ (`self.CountB`) 1)))))))
  (`self.ComputeEffective`))

(fn `UpdateMatch`
  (params (Delta :type "Float (double-precision)"))
  (bind _matchtime (`self.MatchTime`))
  (bind _cycletimer (`self.CycleTimer`))
  (bind _cycleperiod (`self.CyclePeriod`))
  (bind _winscore (`self.WinScore`))
  (bind _returnvalue (>= (`self.ScoreA`) _winscore))
  (set `self.MatchTime` (+ _matchtime Delta))
  (`|ExecutionSequence`
    (:`then_0`
      (if (>= _matchtime (`self.CoreUnlockDelay`))
        (set `self.bCoreUnlocked` true)))
    (:`then_1`
      (if (`self.bCoreUnlocked`)
        (set `self.CycleTimer` (+ (`self.CycleTimer`) Delta))
        (`|ExecutionSequence`
          (:`then_0`
            (if (>= _cycletimer _cycleperiod)
              (`self.UpdateCounts`)
              (set `self.CycleTimer` (- _cycletimer _cycleperiod))
              (`self.PayScore` (`self.PrevOwner`))
              (set `self.CycleIndex` (+ (`self.CycleIndex`) 1))
              (if (or _returnvalue (>= (`self.ScoreB`) _winscore))
                (set `self.bEnded` true)
                (set `self.WinnerTeam` (`KismetMathLibrary.SelectInt` 0 1 _returnvalue))
                (`self.PushHUD` true)
                (`/Game/CODE/UI/UI_ZoneHUD.SetMatchResult` (`self.HUDWidget`) (`self.WinnerTeam`))
                (else
                  (`self.LockOwner`)))))
          (:`then_1`
            (`self.PushHUD` false)))
        (else
          (`self.PushHUD` false))))))

(fn `UserConstructionScript`)
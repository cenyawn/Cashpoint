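; BP_Facility is a capturable objective that registers with BP_CorePOI and reports owner changes to it.
; Each tick samples the player against the zone box and interact radius, driving a four-state machine: idle, hold-to-capture, in-zone countdown, timed ownership.
; A change-gated widget shows prompt, progress and countdown, with a timer turning it yaw-only toward the camera.
; Only player capture (team 0) is implemented, and the cash reward's AddCash call is unwired.
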(event `self.ReceiveBeginPlay`
  (`KismetSystemLibrary.K2_SetTimerDelegate` (delegate `OnFacePromptTimer`) 0.1 true)
  (`self.ResolveRefs` :!label _label)
  (`self.SampleGeometry`)
  (`self.TickState`)
  (`self.RefreshPrompt`))

(event `self.ReceiveTick`
  (params (DeltaSeconds :type "Float (single-precision)"))
  (set `self.FrameDelta` DeltaSeconds)
  (goto _label))

(event `OnFacePromptTimer`
  (bind _returnvalue (`GameplayStatics.GetPlayerCameraManager` 0))
  (bind _promptcomp (`self.PromptComp`))
  (if (not (`self.bPromptSuppressed`))
    (`/Engine/EditorBlueprintResources/StandardMacros.IsValid` _promptcomp
      (:`Is Valid`
        (`/Engine/EditorBlueprintResources/StandardMacros.IsValid` _returnvalue
          (:`Is Valid`
            (`SceneComponent.K2_SetWorldRotation` _promptcomp (`KismetMathLibrary.MakeRotator` 0.0 0.0 (.yaw (`KismetMathLibrary.FindLookAtRotation` (`SceneComponent.K2_GetComponentLocation` _promptcomp) (`PlayerCameraManager.GetCameraLocation` _returnvalue)))) false false)))))))

(fn `AwardCash`
  (if (== (`self.OwnerTeam`) 0)
    (bind _outactors (`GameplayStatics.GetAllActorsOfClass` "/Game/CODE/Player/BP_FPSPlayer.BP_FPSPlayer_C"))
    (if (`KismetArrayLibrary.Array_IsValidIndex` _outactors)
      (bind _asbp_fpsplayer (cast `/Game/CODE/Player/BP_FPSPlayer` (`|GetArrayItem` _outactors))))))

(fn `ColorForTeam`
  (params (Team :type Integer))
  (returns (OutColor :type "LinearColor Structure"))
  (locals (C :type "LinearColor Structure"))
  (if (== Team 0)
    (set `local.C` (make `LinearColor` 0.85 0.1 0.1 1.0))
    (elif (== Team 1)
      (set `local.C` (make `LinearColor` 0.1 0.3 0.95 1.0))
      (else
        (set `local.C` (make `LinearColor` 0.5 0.5 0.5 1.0)))))
  (return (`local.C`)))

(fn `CompleteCapture`
  (set `self.State` 3)
  (set `self.OwnerTeam` (`self.CapturingTeam`))
  (set `self.ActiveRemaining` (`self.ActiveDuration`))
  (set `self.PendingRemaining` 0.0)
  (`self.AwardCash`)
  (`self.NotifyZone`))

(fn `ExpireFacility`
  (set `self.State` 0)
  (set `self.OwnerTeam` 2)
  (set `self.CapturingTeam` 2)
  (set `self.ActiveRemaining` 0.0)
  (`self.NotifyZone`))

(fn `NotifyZone`
  (bind _controlzoneref (`self.ControlZoneRef`))
  (`self.ResolveRefs`)
  (if (`KismetSystemLibrary.IsValid` _controlzoneref)
    (`/Game/CODE/Objective/BP_CorePOI.OnFacilityOwnerChanged` _controlzoneref (`self.FacilityId`) (`self.OwnerTeam`))))

(fn `RefreshPrompt`
  (bind _promptwidget (`self.PromptWidget`))
  (bind _state (`self.State`))
  (bind _lastpromptstate (`self.LastPromptState`))
  (bind _binrange (`self.bInRange`))
  (bind _interactprogress (`self.InteractProgress`))
  (bind _pendingremaining (`self.PendingRemaining`))
  (bind _lastcountdown (`self.LastCountdown`))
  (bind _returnvalue (`KismetMathLibrary.FCeil` _pendingremaining))
  (bind _returnvalue_2 (`KismetMathLibrary.FCeil` (* _interactprogress 20.0)))
  (if (`self.bPromptSuppressed`)
    (if (!= _lastpromptstate -1)
      (`/Game/CODE/UI/UI_FacilityPrompt.SetPrompt` _promptwidget false "")
      (set `self.LastPromptState` -1 :!label _label))
    (elif (`KismetSystemLibrary.IsValid` _promptwidget)
      (if (or (xor _binrange (`self.LastInRange`)) (!= _state _lastpromptstate) (!= _returnvalue_2 (`self.LastProgressPct`)) (!= _returnvalue _lastcountdown))
        (if (== _state 0)
          (if _binrange
            (`/Game/CODE/UI/UI_FacilityPrompt.SetPrompt` _promptwidget true "Hold F to capture")
            (else
              (`/Game/CODE/UI/UI_FacilityPrompt.SetPrompt` _promptwidget false "")))
          (bind _outcolor (`self.ColorForTeam` 2))
          (`/Game/CODE/UI/UI_FacilityPrompt.SetProgress` _promptwidget 0.0 _outcolor)
          (`/Game/CODE/UI/UI_FacilityPrompt.SetCountdown` _promptwidget 0.0 false)
          (set `self.LastPromptState` _state :!label _label_2)
          (set `self.LastInRange` _binrange)
          (set `self.LastProgressPct` _returnvalue_2)
          (elif (== _state 1)
            (bind _outcolor_2 (`self.ColorForTeam` (`self.CapturingTeam`)))
            (`/Game/CODE/UI/UI_FacilityPrompt.SetPrompt` _promptwidget true (`|FormatText` "Capturing {0} / {1} s" (`KismetMathLibrary.FCeil` _interactprogress) (`KismetMathLibrary.FCeil` (`self.InteractHoldTime`))))
            (`/Game/CODE/UI/UI_FacilityPrompt.SetProgress` _promptwidget (/ (`self.InteractProgress`) (`self.InteractHoldTime`)) _outcolor_2)
            (`/Game/CODE/UI/UI_FacilityPrompt.SetCountdown` _promptwidget 0.0 false)
            (goto _label_2)
            (elif (== _state 2)
              (`/Game/CODE/UI/UI_FacilityPrompt.SetPrompt` _promptwidget false "")
              (if (!= _returnvalue _lastcountdown)
                (`/Game/CODE/UI/UI_FacilityPrompt.SetCountdown` _promptwidget _pendingremaining true)
                (set `self.LastCountdown` _returnvalue)
                (goto _label_2)
                (else
                  (goto _label_2)))
              (elif (== _state 3)
                (`/Game/CODE/UI/UI_FacilityPrompt.SetPrompt` _promptwidget false "")
                (`/Game/CODE/UI/UI_FacilityPrompt.SetCountdown` _promptwidget 0.0 false)
                (goto _label_2))))))
      (else
        (goto _label)))))

(fn `ResetFacility`
  (set `self.State` 0)
  (set `self.OwnerTeam` 2)
  (set `self.CapturingTeam` 2)
  (set `self.InteractProgress` 0.0)
  (set `self.PendingRemaining` 0.0)
  (set `self.ActiveRemaining` 0.0)
  (set `self.LastPromptState` -1)
  (set `self.LastCountdown` -1))

(fn `ResolveRefs`
  (bind _controlzoneref (`self.ControlZoneRef`))
  (if (not (`KismetSystemLibrary.IsValid` (`self.ControlZoneRef`)))
    (bind _outactors (`GameplayStatics.GetAllActorsOfClass` "/Game/CODE/Objective/BP_CorePOI.BP_CorePOI_C"))
    (if (`KismetArrayLibrary.Array_IsValidIndex` _outactors)
      (bind _asbp_core_poi (cast `/Game/CODE/Objective/BP_CorePOI` (`|GetArrayItem` _outactors)))
      (set `self.ControlZoneRef` _asbp_core_poi)))
  (if (and (not (`self.bRegistered`)) (`KismetSystemLibrary.IsValid` _controlzoneref))
    (`/Game/CODE/Objective/BP_CorePOI.RegisterFacility` _controlzoneref self)
    (set `self.bRegistered` true))
  (if (not (`KismetSystemLibrary.IsValid` (`self.PromptWidget`)))
    (bind _asui_facility_prompt (cast `/Game/CODE/UI/UI_FacilityPrompt` (`WidgetComponent.GetUserWidgetObject` (`self.PromptComp`))))
    (set `self.PromptWidget` _asui_facility_prompt)))

(fn `SampleGeometry`
  (bind _returnvalue (`self.K2_GetActorLocation`))
  (bind _returnvalue_2 (`GameplayStatics.GetPlayerCharacter` 0))
  (bind _playerref (`self.PlayerRef`))
  (bind _returnvalue_3 (`self.K2_GetActorLocation` _playerref))
  (bind _returnvalue_4 (and (and (<= (`KismetMathLibrary.Abs` (.x (- _returnvalue_3 (`self.ZoneCenter`)))) (.x (`self.ControlExtent`))) (<= (`KismetMathLibrary.Abs` (.y (- _returnvalue_3 (`self.ZoneCenter`)))) (.y (`self.ControlExtent`)))) (<= (`KismetMathLibrary.Abs` (.z (- _returnvalue_3 (`self.ZoneCenter`)))) (.z (`self.ControlExtent`)))))
  (set `self.bInRange` false)
  (set `self.bInZone` false)
  (set `self.bInteractHeldLocal` false)
  (if (not (`KismetSystemLibrary.IsValid` _playerref))
    (`/Engine/EditorBlueprintResources/StandardMacros.IsValid` _returnvalue_2
      (:`Is Valid`
        (bind _asbp_fpsplayer (cast `/Game/CODE/Player/BP_FPSPlayer` _returnvalue_2))
        (set `self.PlayerRef` _asbp_fpsplayer))))
  (set `self.bInteractHeldLocal` (`/Game/CODE/Player/BP_FPSPlayer.bInteractHeld` _playerref))
  (set `self.bPromptSuppressed` (or (`/Game/CODE/Combat/BP_HealthComponent.bDead` (`/Game/CODE/Player/BP_FPSPlayer.HealthComponent` _playerref)) (`/Game/CODE/Player/BP_FPSPlayer.bUIOpen` _playerref)))
  (set `self.bInZone` _returnvalue_4)
  (set `self.bInRange` (and _returnvalue_4 (and (<= (`KismetMathLibrary.Vector_Distance2D` _returnvalue_3 _returnvalue) (`self.InteractRadius`)) (<= (`KismetMathLibrary.Abs` (.z (- _returnvalue_3 _returnvalue))) (`self.InteractZRange`))))))

(fn `TickState`
  (bind _state (`self.State`))
  (bind _returnvalue (and (`self.bInRange`) (`self.bInteractHeldLocal`)))
  (if (== _state 3)
    (set `self.ActiveRemaining` (- (`self.ActiveRemaining`) (`self.FrameDelta`)))
    (if (<= (`self.ActiveRemaining`) 0.0)
      (`self.ExpireFacility`))
    (elif (== _state 2)
      (if (`self.bInZone`)
        (set `self.PendingRemaining` (- (`self.PendingRemaining`) (`self.FrameDelta`)))
        (if (and _returnvalue (!= (`self.CapturingTeam`) 0))
          (set `self.CapturingTeam` 0)
          (set `self.PendingRemaining` (`self.CaptureWaitTime`)))
        (if (<= (`self.PendingRemaining`) 0.0)
          (`self.CompleteCapture`))
        (else
          (set `self.InteractProgress` 0.0)
          (set `self.PendingRemaining` 0.0)
          (set `self.CapturingTeam` 2)
          (set `self.State` 0)))
      (elif (== _state 1)
        (if _returnvalue
          (set `self.InteractProgress` (+ (`self.InteractProgress`) (`self.FrameDelta`)))
          (if (>= (`self.InteractProgress`) (`self.InteractHoldTime`))
            (set `self.State` 2)
            (set `self.PendingRemaining` (`self.CaptureWaitTime`))
            (set `self.InteractProgress` (`self.InteractHoldTime`)))
          (else
            (set `self.InteractProgress` 0.0)
            (set `self.State` 0)))
        (elif (== _state 0)
          (if _returnvalue
            (set `self.CapturingTeam` 0)
            (set `self.State` 1)))))))

(fn `UserConstructionScript`)
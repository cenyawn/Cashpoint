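; Shop component that holds a weapon catalog for the game's economy and tracks which items are owned.
; On BeginPlay, InitCatalog fills parallel arrays with three hardcoded weapons if the catalog is empty, with only the MCX-VIRTUS enabled.
; Lookup functions resolve an item ID to its index for price, availability and grant class path, with bounds-checked defaults.
; Ownership lives in a separate ID list, exportable as per-item flags; purchasing and spawning are not handled here.
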(event `self.ReceiveBeginPlay`
  (`self.InitCatalog`))

(fn `GetGrantClass`
  (params (ItemId :type Name))
  (returns (Return :type String))
  (locals (SOut :type String))
  (bind _itemgrantclass (`self.ItemGrantClass`))
  (bind _returnvalue (`KismetArrayLibrary.Array_Find` (`self.ItemIds`) ItemId))
  (set `local.SOut` "")
  (if (and (>= _returnvalue 0) (< _returnvalue (`KismetArrayLibrary.Array_Length` _itemgrantclass)))
    (set `local.SOut` (`|GetArrayItem` _itemgrantclass _returnvalue)))
  (return (`local.SOut`)))

(fn `GetItemIndex`
  (params (ItemId :type Name))
  (returns (Return :type Integer))
  (return (`KismetArrayLibrary.Array_Find` (`self.ItemIds`) ItemId)))

(fn `GetItemPrice`
  (params (ItemId :type Name))
  (returns (Return :type Integer))
  (locals (POut :type Integer) (POut_0 :type Integer))
  (bind _itemprices (`self.ItemPrices`))
  (bind _returnvalue (`KismetArrayLibrary.Array_Find` (`self.ItemIds`) ItemId))
  (set `local.POut` 0)
  (if (and (>= _returnvalue 0) (< _returnvalue (`KismetArrayLibrary.Array_Length` _itemprices)))
    (set `local.POut` (`|GetArrayItem` _itemprices _returnvalue)))
  (return (`local.POut`)))

(fn `GetOwnedFlags`
  (returns (Return :type "Array of Boolean"))
  (locals (Flags :type "Array of Boolean"))
  (`KismetArrayLibrary.Array_Clear` (`local.Flags`))
  (for _array_element (`self.ItemIds`)
    (`KismetArrayLibrary.Array_Add` (`local.Flags`) (`KismetArrayLibrary.Array_Contains` (`self.OwnedIds`) _array_element)))
  (return (`local.Flags`)))

(fn `InitCatalog`
  (bind _itemids (`self.ItemIds`))
  (bind _itemnames (`self.ItemNames`))
  (bind _itemtypelabels (`self.ItemTypeLabels`))
  (bind _itemcategories (`self.ItemCategories`))
  (bind _itemprices (`self.ItemPrices`))
  (bind _itemdescriptions (`self.ItemDescriptions`))
  (bind _itemstats (`self.ItemStats`))
  (bind _itemenabled (`self.ItemEnabled`))
  (bind _itemgrantclass (`self.ItemGrantClass`))
  (if (== (`KismetArrayLibrary.Array_Length` _itemids) 0)
    (`KismetArrayLibrary.Array_Add` _itemids "rifle_mcx")
    (`KismetArrayLibrary.Array_Add` _itemids "smg_uzi")
    (`KismetArrayLibrary.Array_Add` _itemids "pistol_deagle")
    (`KismetArrayLibrary.Array_Add` _itemnames "MCX-VIRTUS")
    (`KismetArrayLibrary.Array_Add` _itemnames "UZI")
    (`KismetArrayLibrary.Array_Add` _itemnames "DESERT EAGLE")
    (`KismetArrayLibrary.Array_Add` _itemtypelabels "RIFLE")
    (`KismetArrayLibrary.Array_Add` _itemtypelabels "SMG")
    (`KismetArrayLibrary.Array_Add` _itemtypelabels "PISTOL")
    (`KismetArrayLibrary.Array_Add` _itemcategories "Weapon")
    (`KismetArrayLibrary.Array_Add` _itemcategories "Weapon")
    (`KismetArrayLibrary.Array_Add` _itemcategories "Weapon")
    (`KismetArrayLibrary.Array_Add` _itemprices 2700)
    (`KismetArrayLibrary.Array_Add` _itemprices)
    (`KismetArrayLibrary.Array_Add` _itemprices 700)
    (`KismetArrayLibrary.Array_Add` _itemdescriptions "Standard issue assault rifle. 30-round magazine.")
    (`KismetArrayLibrary.Array_Add` _itemdescriptions "Coming soon.")
    (`KismetArrayLibrary.Array_Add` _itemdescriptions "Coming soon.")
    (`KismetArrayLibrary.Array_Add` _itemstats "DMG 25   MAG 30   RATE 0.1")
    (`KismetArrayLibrary.Array_Add` _itemstats "COMING SOON")
    (`KismetArrayLibrary.Array_Add` _itemstats "COMING SOON")
    (`KismetArrayLibrary.Array_Add` _itemenabled true)
    (`KismetArrayLibrary.Array_Add` _itemenabled)
    (`KismetArrayLibrary.Array_Add` _itemenabled)
    (`KismetArrayLibrary.Array_Add` _itemgrantclass "/Game/CODE/Weapon/BP_Virtus.BP_Virtus_C")
    (`KismetArrayLibrary.Array_Add` _itemgrantclass)
    (`KismetArrayLibrary.Array_Add` _itemgrantclass)))

(fn `IsItemEnabled`
  (params (ItemId :type Name))
  (returns (Return :type Boolean))
  (locals (BOut :type Boolean))
  (bind _itemenabled (`self.ItemEnabled`))
  (bind _returnvalue (`KismetArrayLibrary.Array_Find` (`self.ItemIds`) ItemId))
  (set `local.BOut` false)
  (if (and (>= _returnvalue 0) (< _returnvalue (`KismetArrayLibrary.Array_Length` _itemenabled)))
    (set `local.BOut` (`|GetArrayItem` _itemenabled _returnvalue)))
  (return (`local.BOut`)))

(fn `IsItemOwned`
  (params (ItemId :type Name))
  (returns (Return :type Boolean))
  (return (`KismetArrayLibrary.Array_Contains` (`self.OwnedIds`) ItemId)))

(fn `MarkOwned`
  (params (ItemId :type Name))
  (`KismetArrayLibrary.Array_AddUnique` (`self.OwnedIds`) ItemId))

(fn `ResetOwned`
  (`KismetArrayLibrary.Array_Clear` (`self.OwnedIds`)))
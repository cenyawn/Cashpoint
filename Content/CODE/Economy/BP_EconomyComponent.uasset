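; Economy component that holds an actor's Cash balance, starting from StartingCash and able to reset to it.
; AddCash clamps the total between zero and MaxCash, and AddKillReward uses it to pay a fixed kill bounty.
; TrySpend and SpendCash deduct only when affordable, though SpendCash re-tests affordability after deducting for its return value.
; Balance changes fire OnCashChanged so listeners can follow the total.
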(event `self.ReceiveBeginPlay`
  (set `self.Cash` (`self.StartingCash`))
  (`self.OnCashChanged` (`self.Cash`)))

(fn `AddCash`
  (params (Amount :type Integer))
  (returns (Return :type Integer))
  (bind _cash (`self.Cash`))
  (set `self.Cash` (`KismetMathLibrary.Clamp` (+ (`self.Cash`) Amount) 0 (`self.MaxCash`)))
  (`self.OnCashChanged` _cash)
  (return _cash))

(fn `AddKillReward`
  (returns (Return :type Integer))
  (bind _return (`self.AddCash` (`self.KillRewardCash`)))
  (return _return))

(fn `CanAfford`
  (params (Amount :type Integer))
  (returns (Return :type Boolean))
  (return (>= (`self.Cash`) Amount)))

(fn `GetCash`
  (returns (Return :type Integer))
  (return (`self.Cash`)))

(fn `ResetToStart`
  (set `self.Cash` (`self.StartingCash`))
  (`self.OnCashChanged` (`self.Cash`)))

(fn `SpendCash`
  (params (Amount :type Integer))
  (returns (Return :type Boolean))
  (bind _returnvalue (>= (`self.Cash`) Amount))
  (if _returnvalue
    (set `self.Cash` (- (`self.Cash`) Amount))
    (`self.OnCashChanged` (`self.Cash`))
    (return _returnvalue)
    (else
      (return false))))

(fn `TrySpend`
  (params (Amount :type Integer))
  (returns (Return :type Boolean))
  (locals (bOk :type Boolean))
  (if (<= Amount 0)
    (set `local.bOk` true)
    (elif (>= (`self.Cash`) Amount)
      (set `self.Cash` (`KismetMathLibrary.Clamp` (- (`self.Cash`) Amount) 0 (`self.MaxCash`)))
      (`self.OnCashChanged` (`self.Cash`))
      (set `local.bOk` true)))
  (return (`local.bOk`)))
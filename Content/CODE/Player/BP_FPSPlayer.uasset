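; First-person player character with Enhanced Input movement, aiming with FOV zoom, weapon firing, and a merchant shop.
; Tick aligns the arm to control rotation and derives an Idle/Walk/Run/Aim state that sets walk speed.
; Health and economy components feed the HUD; death disables control, and BP_CorePOI provides match reset, with ResetForNewMatch restoring the player at spawn.
; TryPurchase handles shop transactions, but HandlePurchaseRequested only reports "Unavailable" without calling it.
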(event `EnhancedInput|/Game/CODE/Player/System/Input/IA_Run`
  (params (ActionValue :type Boolean) (ElapsedSeconds :type "Float (double-precision)") (TriggeredSeconds :type "Float (double-precision)") (InputAction :type "InputAction Object Reference" :default "/Game/CODE/Player/System/Input/IA_Run.IA_Run"))
  ; 角色能力系统
  (:`Triggered`
    (set `self.Want to Run` true))
  (:`Completed`
    (set `self.Want to Run` false)))

(event `self.ReceiveTick`
  (params (DeltaSeconds :type "Float (single-precision)"))
  (bind (_returnvalue_roll _returnvalue_pitch _returnvalue_yaw) (`KismetMathLibrary.BreakRotator` (`self.GetControlRotation`)))
  ; 角色能力系统
  (`SceneComponent.K2_SetWorldRotation` (`self.Arm`) (`KismetMathLibrary.MakeRotator` 0.0 _returnvalue_pitch _returnvalue_yaw) false false)
  (`self.UpdatePlayerState`)
  (`self.UpdateMoveSpeed`))

(event `self.ReceiveBeginPlay`
  (bind _economycomponent (`self.EconomyComponent`))
  (bind _mainui (`self.MainUi`))
  (bind _healthcomponent (`self.HealthComponent`))
  ; 激活操作系统
  (set `self.RespawnPoint` (`self.K2_GetActorLocation`))
  (set `self.RespawnYaw` (.yaw (`self.K2_GetActorRotation`)))
  (bind _returnvalue (`|CreateWidget` "/Game/CODE/UI/UI_MainUi.UI_MainUi_C"))
  (bind _output_get (set `self.MainUi` _returnvalue))
  (`UserWidget.AddToViewport` _output_get 0)
  (if (`KismetSystemLibrary.IsValid` _mainui)
    (`/Game/CODE/UI/UI_MainUi.UpdateHealth` _mainui (`/Game/CODE/Combat/BP_HealthComponent.Health` _healthcomponent) (`/Game/CODE/Combat/BP_HealthComponent.MaxHealth` _healthcomponent))
    (if (`KismetSystemLibrary.IsValid` _mainui)
      (`/Game/CODE/UI/UI_MainUi.UpdateCash` _mainui (`/Game/CODE/Economy/BP_EconomyComponent.Cash` _economycomponent))
      (add `/Game/CODE/Combat/BP_HealthComponent.OnDeath` (`self.HealthComponent`) (delegate `HandleDeath`) :!label _label)
      (add `/Game/CODE/Economy/BP_EconomyComponent.OnCashChanged` _economycomponent (`|CreateDelegate` self :!event `OnCashChanged`))
      (bind _asplayer_controller (cast `PlayerController` (`self.GetController`)))
      (`EnhancedInputSubsystemInterface.AddMappingContext` (pcsubsystem `EnhancedInputLocalPlayerSubsystem` _asplayer_controller) "/Game/CODE/Player/System/Input/IMC_FPSInput.IMC_FPSInput" 0 (struct))
      (`self.SpawnWeapon` "/Game/CODE/Weapon/BP_Virtus.BP_Virtus_C")
      (`self.UpdateDefaultFOV`)
      (bind _outactors (`GameplayStatics.GetAllActorsOfClass` "/Game/CODE/Objective/BP_CorePOI.BP_CorePOI_C"))
      (if (`KismetArrayLibrary.Array_IsValidIndex` _outactors)
        (bind _asbp_core_poi (cast `/Game/CODE/Objective/BP_CorePOI` (`|GetArrayItem` _outactors)))
        (`/Game/CODE/Objective/BP_CorePOI.SetHUD` _asbp_core_poi (`/Game/CODE/UI/UI_MainUi.ZoneHUD` _mainui))
        (add `/Game/CODE/Objective/BP_CorePOI.OnMatchReset` _asbp_core_poi (`|CreateDelegate` :!event `ResetForNewMatch`))))
    (else
      (goto _label))))

(event `self.HealthComponent.OnHealthChanged`
  (params (Health :type "Float (double-precision)") (MaxHealth :type "Float (double-precision)"))
  (bind _mainui (`self.MainUi`))
  ; 激活操作系统
  (if (`KismetSystemLibrary.IsValid` _mainui)
    (`/Game/CODE/UI/UI_MainUi.UpdateHealth` _mainui Health MaxHealth)))

(event `EnhancedInput|/Game/CODE/Player/System/Input/IA_Move`
  (params (ActionValue :type "Vector2D Structure") (ElapsedSeconds :type "Float (double-precision)") (TriggeredSeconds :type "Float (double-precision)") (InputAction :type "InputAction Object Reference" :default "/Game/CODE/Player/System/Input/IA_Move.IA_Move"))
  (bind (_x _y) (`KismetMathLibrary.BreakVector2D` ActionValue))
  (bind (_returnvalue_roll _returnvalue_pitch _returnvalue_yaw) (`KismetMathLibrary.BreakRotator` (`self.GetControlRotation`)))
  (bind (_returnvalue_roll_2 _returnvalue_pitch_2 _returnvalue_yaw_2) (`KismetMathLibrary.BreakRotator` (`self.GetControlRotation`)))
  ; 角色移动
  (:`Triggered`
    (bind _output_get (set `self.Move X` _x))
    (`self.AddMovementInput` (`KismetMathLibrary.GetForwardVector` (`KismetMathLibrary.MakeRotator` 0.0 0.0 _returnvalue_yaw_2)) _output_get)
    (bind _output_get_2 (set `self.Move Y` _y))
    (`self.AddMovementInput` (`KismetMathLibrary.GetRightVector` (`KismetMathLibrary.MakeRotator` 0.0 0.0 _returnvalue_yaw)) _output_get_2))
  (:`Completed`
    (set `self.Move X` 0.0)
    (set `self.Move Y` 0.0)))

(event `HandleDeath`
  (`self.CloseMerchantShop`)
  (set `self.IsDead` true)
  (if (`KismetSystemLibrary.IsValid` (`self.CurrentWeapon`))
    (`/Game/CODE/Weapon/Base/BP_WeaponBase.StopFire` (`self.CurrentWeapon`)))
  (set `self.IsFiring` false)
  (bind _asplayer_controller (cast `PlayerController` (`self.GetController`))
    (:`then`
      (`self.DisableInput` _asplayer_controller))
    (:`CastFailed`
      _))
  (`CharacterMovementComponent.DisableMovement` (`self.CharacterMovement`))
  (set `self.Want to Run` false)
  (set `self.Want to Aim` false)
  (set `CameraComponent.FieldOfView` (`self.DefaultFov`) (`self.Camera`))
  (`KismetSystemLibrary.K2_ClearAndInvalidateTimerHandle` (`self.OutFOVHandle`))
  (set `self.bCanBeDamaged` false))

(event `EnhancedInput|/Game/CODE/Player/System/Input/IA_Look`
  (params (ActionValue :type "Vector2D Structure") (ElapsedSeconds :type "Float (double-precision)") (TriggeredSeconds :type "Float (double-precision)") (InputAction :type "InputAction Object Reference" :default "/Game/CODE/Player/System/Input/IA_Look.IA_Look"))
  (bind (_x _y) (`KismetMathLibrary.BreakVector2D` ActionValue))
  ; 角色视角
  (:`Triggered`
    (`self.AddControllerYawInput` (* _x (`self.UpdateScopeSensitivity`) (`self.MouseSensitivity`)))
    (`self.AddControllerPitchInput` (* _y (`self.UpdateScopeSensitivity`) (`self.MouseSensitivity`)))))

(event `EnhancedInput|/Game/CODE/Player/System/Input/IA_Aim`
  (params (ActionValue :type Boolean) (ElapsedSeconds :type "Float (double-precision)") (TriggeredSeconds :type "Float (double-precision)") (InputAction :type "InputAction Object Reference" :default "/Game/CODE/Player/System/Input/IA_Aim.IA_Aim"))
  (bind _camera (`self.Camera`))
  (:`Triggered`
    (if (`KismetSystemLibrary.IsValid` (`self.CurrentWeapon`))
      (set `self.Want to Aim` true)
      (`CameraComponent.SetFieldOfView` _camera (`KismetMathLibrary.FInterpTo` (`CameraComponent.FieldOfView` _camera) 75.0 (`GameplayStatics.GetWorldDeltaSeconds`) 8.0))
      (`KismetSystemLibrary.K2_ClearAndInvalidateTimerHandle` (`self.OutFOVHandle`))))
  (:`Completed`
    (set `self.Want to Aim` false)
    (bind _returnvalue (`KismetSystemLibrary.K2_SetTimerDelegate` (delegate `OutFov`) (`GameplayStatics.GetWorldDeltaSeconds`) true))
    (set `self.OutFOVHandle` _returnvalue)))

(event `OutFov`
  (bind _camera (`self.Camera`))
  (bind _fieldofview (`CameraComponent.FieldOfView` _camera))
  (`CameraComponent.SetFieldOfView` _camera (`KismetMathLibrary.FInterpTo` _fieldofview (`self.DefaultFov`) (`GameplayStatics.GetWorldDeltaSeconds`) 8.0))
  (if (`KismetMathLibrary.NearlyEqual_FloatFloat` _fieldofview (`self.DefaultFov`) 0.1)
    (`KismetSystemLibrary.K2_ClearAndInvalidateTimerHandle` (`self.OutFOVHandle`))))

(event `EnhancedInput|/Game/CODE/Player/System/Input/IA_Fire`
  (params (ActionValue :type Boolean) (ElapsedSeconds :type "Float (double-precision)") (TriggeredSeconds :type "Float (double-precision)") (InputAction :type "InputAction Object Reference" :default "/Game/CODE/Player/System/Input/IA_Fire.IA_Fire"))
  (:`Started`
    (if (not (`self.bUIOpen`))
      (if (`self.IsFiring`)
        _
        (elif (`self.IsDead`)
          _
          (elif (`|EnumInequality` (`self.E_PlayerState`) "NewEnumerator2")
            (if (`KismetSystemLibrary.IsValid` (`self.CurrentWeapon`))
              (message `/Game/CODE/BlueprintInterface/BI_Fire.StartWeaponFire` (`self.CurrentWeapon`) self)))))))
  (:`Completed`
    (if (`KismetSystemLibrary.IsValid` (`self.CurrentWeapon`))
      (`/Game/CODE/Weapon/Base/BP_WeaponBase.StopFire` (`self.CurrentWeapon`)))
    (set `self.IsFiring` false)))

(event `EnhancedInput|/Game/CODE/Player/System/Input/IA_Reload`
  (params (ActionValue :type Boolean) (ElapsedSeconds :type "Float (double-precision)") (TriggeredSeconds :type "Float (double-precision)") (InputAction :type "InputAction Object Reference" :default "/Game/CODE/Player/System/Input/IA_Reload.IA_Reload"))
  (:`Started`
    (`/Game/CODE/Weapon/Base/BP_WeaponBase.Reload` (`self.CurrentWeapon`) self)))

(event `EnhancedInput|/Game/CODE/Player/System/Input/IA_Reset`
  (params (ActionValue :type Boolean) (ElapsedSeconds :type "Float (double-precision)") (TriggeredSeconds :type "Float (double-precision)") (InputAction :type "InputAction Object Reference" :default "/Game/CODE/Player/System/Input/IA_Reset.IA_Reset"))
  (:`Started`
    (bind _outactors (`GameplayStatics.GetAllActorsOfClass` "/Game/CODE/Objective/BP_CorePOI.BP_CorePOI_C"))
    (if (`KismetArrayLibrary.Array_IsValidIndex` _outactors)
      (bind _asbp_core_poi (cast `/Game/CODE/Objective/BP_CorePOI` (`|GetArrayItem` _outactors)))
      (`/Game/CODE/Objective/BP_CorePOI.ResetMatch` _asbp_core_poi))))

(event `EnhancedInput|/Game/CODE/Player/System/Input/IA_Interact`
  (params (ActionValue :type Boolean) (ElapsedSeconds :type "Float (double-precision)") (TriggeredSeconds :type "Float (double-precision)") (InputAction :type "InputAction Object Reference" :default "/Game/CODE/Player/System/Input/IA_Interact.IA_Interact"))
  (:`Started`
    (set `self.bInteractHeld` true))
  (:`Completed`
    (set `self.bInteractHeld` false)))

(fn `CloseMerchantShop`
  (bind _shopwidget (`self.ShopWidget`))
  (if (`self.bUIOpen`)
    (set `self.bUIOpen` false)
    (bind _asplayer_controller (cast `PlayerController` (`self.GetController`)))
    (if (`KismetSystemLibrary.IsValid` _shopwidget)
      (set `Widget.Visibility` (enumliteral `ESlateVisibility` "Collapsed") _shopwidget))
    (`WidgetBlueprintLibrary.SetInputMode_GameOnly` _asplayer_controller)
    (set `PlayerController.bShowMouseCursor` false _asplayer_controller)
    (`Controller.SetIgnoreMoveInput` _asplayer_controller false)
    (`Controller.SetIgnoreLookInput` _asplayer_controller false)))

(fn `GrantWeapon`
  (returns (Return :type "/Game/CODE/Weapon/Base/BP_WeaponBase Object Reference"))
  (if (not (`KismetSystemLibrary.IsValid` (`self.CurrentWeapon`)))
    (`self.SpawnWeapon` "/Game/CODE/Weapon/BP_Virtus.BP_Virtus_C"))
  (return (`self.CurrentWeapon`)))

(fn `HandlePurchaseRequested`
  (params (ItemId :type Name))
  (bind _shopwidget (`self.ShopWidget`))
  (if (`KismetSystemLibrary.IsValid` _shopwidget)
    (bind _return (`/Game/CODE/Economy/BP_ShopComponent.GetItemPrice` (`self.ShopComponent`) ItemId))
    (`/Game/CODE/UI/UI_Shop.ShowPurchaseResult` _shopwidget "Unavailable" _return)))

(fn `OnCashChanged`
  (params (NewCash :type Integer))
  (bind _mainui (`self.MainUi`))
  (if (`KismetSystemLibrary.IsValid` _mainui)
    (`/Game/CODE/UI/UI_MainUi.UpdateCash` _mainui NewCash)))

(fn `OpenMerchantShop`
  (bind _shopwidget (`self.ShopWidget`))
  (bind _shopcomponent (`self.ShopComponent`))
  (bind _shopwidget_2 (`self.ShopWidget`))
  (bind _shopwidget_3 (`self.ShopWidget`))
  (bind _currentweapon (`self.CurrentWeapon`))
  (if (not (`self.bUIOpen`))
    (bind _asplayer_controller (cast `PlayerController` (`self.GetController`)))
    (if (`KismetSystemLibrary.IsValid` _shopwidget_2)
      (set `Widget.Visibility` (enumliteral `ESlateVisibility` "Visible") _shopwidget_2)
      (else
        (bind _returnvalue (`|CreateWidget` "/Game/CODE/UI/UI_Shop.UI_Shop_C" _asplayer_controller))
        (set `self.ShopWidget` _returnvalue)
        (`UserWidget.AddToViewport` _returnvalue 10)
        (add `/Game/CODE/UI/UI_Shop.OnCloseClicked` _returnvalue (`|CreateDelegate` :!event `CloseMerchantShop`))
        (add `/Game/CODE/UI/UI_Shop.OnPurchaseRequested` _shopwidget (`|CreateDelegate` :!event `HandlePurchaseRequested`))
        (bind _return (`/Game/CODE/Economy/BP_EconomyComponent.GetCash` (`self.EconomyComponent`)))
        (bind _return_2 (`/Game/CODE/Economy/BP_ShopComponent.GetOwnedFlags` _shopcomponent))
        (`/Game/CODE/UI/UI_Shop.OpenShop` _shopwidget (`/Game/CODE/Economy/BP_ShopComponent.ItemIds` _shopcomponent) (`/Game/CODE/Economy/BP_ShopComponent.ItemNames` _shopcomponent) (`/Game/CODE/Economy/BP_ShopComponent.ItemTypeLabels` _shopcomponent) (`/Game/CODE/Economy/BP_ShopComponent.ItemCategories` _shopcomponent) (`/Game/CODE/Economy/BP_ShopComponent.ItemPrices` _shopcomponent) (`/Game/CODE/Economy/BP_ShopComponent.ItemDescriptions` _shopcomponent) (`/Game/CODE/Economy/BP_ShopComponent.ItemStats` _shopcomponent) (`/Game/CODE/Economy/BP_ShopComponent.ItemEnabled` _shopcomponent) _return_2 _return)))
    (bind _return_3 (`/Game/CODE/Economy/BP_EconomyComponent.GetCash` (`self.EconomyComponent`)))
    (`/Game/CODE/UI/UI_Shop.UpdateCash` _shopwidget_3 _return_3)
    (`WidgetBlueprintLibrary.SetInputMode_GameAndUIEx` _asplayer_controller _shopwidget_3 "DoNotLock" false)
    (set `PlayerController.bShowMouseCursor` true _asplayer_controller)
    (`Controller.SetIgnoreMoveInput` _asplayer_controller true)
    (`Controller.SetIgnoreLookInput` _asplayer_controller true)
    (if (`KismetSystemLibrary.IsValid` _currentweapon)
      (`/Game/CODE/Weapon/Base/BP_WeaponBase.StopFire` _currentweapon))
    (set `self.bUIOpen` true)))

(fn `ResetForNewMatch`
  (bind _economycomponent (`self.EconomyComponent`))
  (bind _shopcomponent (`self.ShopComponent`))
  (bind _shopwidget (`self.ShopWidget`))
  (bind _charactermovement (`self.CharacterMovement`))
  (`|ExecutionSequence`
    (:`then_0`
      (`self.CloseMerchantShop`)
      (`/Game/CODE/Economy/BP_EconomyComponent.ResetToStart` _economycomponent)
      (`/Game/CODE/Economy/BP_ShopComponent.ResetOwned` _shopcomponent)
      (if (`KismetSystemLibrary.IsValid` _shopwidget)
        (bind _return (`/Game/CODE/Economy/BP_EconomyComponent.GetCash` _economycomponent))
        (bind _return_2 (`/Game/CODE/Economy/BP_ShopComponent.GetOwnedFlags` _shopcomponent))
        (`/Game/CODE/UI/UI_Shop.UpdateCash` _shopwidget _return)
        (`/Game/CODE/UI/UI_Shop.RefreshOwnership` _shopwidget _return_2)))
    (:`then_1`
      (`MovementComponent.StopMovementImmediately` _charactermovement)
      (`self.K2_SetActorLocationAndRotation` (`self.RespawnPoint`) (`KismetMathLibrary.MakeRotator` 0.0 0.0 (`self.RespawnYaw`)) false true)
      (`/Game/CODE/Combat/BP_HealthComponent.ResetHealth` (`self.HealthComponent`))
      (set `self.bCanBeDamaged` true)
      (set `self.IsDead` false)
      (`self.SetActorHiddenInGame` false)
      (`CharacterMovementComponent.SetMovementMode` _charactermovement "MOVE_Walking" 0)
      (bind _asplayer_controller (cast `PlayerController` (`self.GetController`)))
      (`self.EnableInput` _asplayer_controller)
      (if (not (`KismetSystemLibrary.IsValid` (`self.CurrentWeapon`)))
        (`self.SpawnWeapon` "/Game/CODE/Weapon/BP_Virtus.BP_Virtus_C")))))

(fn `SpawnWeapon`
  (params (Class :type "Actor Class Reference"))
  (bind _returnvalue (`|SpawnActorFromClass` Class (`KismetMathLibrary.MakeTransform` (0.0 0.0 0.0)) "Undefined" "MultiplyWithRoot" self null))
  (bind _asbp_weapon_base (cast `/Game/CODE/Weapon/Base/BP_WeaponBase` _returnvalue))
  (bind _output_get (set `self.CurrentWeapon` _asbp_weapon_base))
  (`self.K2_AttachToComponent` _output_get (`self.Arm`) "None" "KeepRelative" "KeepRelative" "KeepRelative" true))

(fn `ToggleMerchantShop`
  (if (`self.bUIOpen`)
    (`self.CloseMerchantShop`)
    (else
      (`self.OpenMerchantShop`))))

(fn `TryPurchase`
  (params (ItemId :type Name))
  (returns (bOk :type Boolean) (ResultCode :type Name))
  (locals (OkOut :type Boolean) (CodeOut :type Name))
  (bind _shopcomponent (`self.ShopComponent`))
  (bind _economycomponent (`self.EconomyComponent`))
  (set `local.OkOut` false)
  (set `local.CodeOut` "Unavailable")
  (bind _return (`/Game/CODE/Economy/BP_ShopComponent.GetItemIndex` _shopcomponent ItemId))
  (if (not (< _return 0))
    (bind _return_2 (`/Game/CODE/Economy/BP_ShopComponent.IsItemEnabled` _shopcomponent ItemId))
    (if (not (not _return_2))
      (bind _return_3 (`/Game/CODE/Economy/BP_ShopComponent.IsItemOwned` _shopcomponent ItemId))
      (if _return_3
        (set `local.CodeOut` "Owned")
        (elif (`/Game/CODE/Combat/BP_HealthComponent.bDead` (`self.HealthComponent`))
          (set `local.CodeOut` "Failed")
          (else
            (bind _return_4 (`/Game/CODE/Economy/BP_ShopComponent.GetItemPrice` _shopcomponent ItemId))
            (bind _return_5 (`/Game/CODE/Economy/BP_EconomyComponent.TrySpend` _economycomponent _return_4))
            (if _return_5
              (set `local.CodeOut` "NoFunds")
              (else
                (bind _return_6 (`/Game/CODE/Economy/BP_ShopComponent.GetGrantClass` _shopcomponent ItemId))
                (if (not (`KismetStringLibrary.IsEmpty` _return_6))
                  (bind _return_7 (`self.GrantWeapon`))
                  (if (not (`KismetSystemLibrary.IsValid` _return_7))
                    (`/Game/CODE/Economy/BP_EconomyComponent.AddCash` _economycomponent _return_4)
                    (set `local.CodeOut` "Failed")
                    (else
                      (`/Game/CODE/Economy/BP_ShopComponent.MarkOwned` _shopcomponent ItemId)
                      (set `local.OkOut` true :!label _label)
                      (set `local.CodeOut` "Success")))
                  (else
                    (`/Game/CODE/Economy/BP_ShopComponent.MarkOwned` _shopcomponent ItemId)
                    (goto _label))))))))))
  (return (`local.OkOut`) (`local.CodeOut`)))

(fn `UpdateDefaultFOV`
  (set `self.DefaultFov` (`CameraComponent.FieldOfView` (`self.Camera`))))

(fn `UpdateMoveSpeed`
  (set `CharacterMovementComponent.MaxWalkSpeed` (select `/Game/CODE/Player/System/Enum/E_PlayerState` (`self.E_PlayerState`) :`NewEnumerator0` 400.0 :`NewEnumerator1` 400.0 :`NewEnumerator2` 800.0 :`NewEnumerator3` 265.0 :!type "Float (single-precision)") (`self.CharacterMovement`)))

(fn `UpdatePlayerState`
  (if (`self.Want to Aim`)
    (set `self.E_PlayerState` "NewEnumerator3")
    (elif (> (`self.Move X`) 0.0)
      (if (`self.Want to Run`)
        (set `self.E_PlayerState` "NewEnumerator2")
        (else
          (set `self.E_PlayerState` "NewEnumerator1")))
      (elif (> (`KismetMathLibrary.VSize` (`MovementComponent.Velocity` (`self.CharacterMovement`))) 0.0)
        (set `self.E_PlayerState` "NewEnumerator1")
        (else
          (set `self.E_PlayerState` "NewEnumerator0"))))))

(fn `UpdateScopeSensitivity`
  (returns (OutSentivity :type "Float (double-precision)"))
  (return (select `/Game/CODE/Player/System/Enum/E_PlayerState` (`self.E_PlayerState`) :`NewEnumerator0` 1.0 :`NewEnumerator1` 1.0 :`NewEnumerator2` 1.0 :`NewEnumerator3` 1.0)))

(fn `UserConstructionScript`)
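; Base weapon actor for a first-person player, handling automatic fire, ammo and reload, with MCX Virtus assets hardcoded.
; A looping timer drives each shot: state-based arm and weapon montages, muzzle flash, casing, recoil and HUD update.
; Camera line traces apply point damage, then spawn blood for pawns or surface-specific effects and decals otherwise.
; WeaponState gates firing and reload montages; ReloadAmmo, not called here, refills the magazine from reserve.
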(event `/Game/CODE/BlueprintInterface/BI_Fire.StartWeaponFire`
  (params (Player :type "/Game/CODE/Player/BP_FPSPlayer Object Reference"))
  (set `self.Player` Player)
  (switch `/Game/CODE/Player/System/Enum/E_WeaponState` (`self.WeaponState`)
    (:`NewEnumerator0`
      (if (> (`self.CurrentAmmo`) 0)
        (`self.FireInternal`)
        (bind _returnvalue (`KismetSystemLibrary.K2_SetTimerDelegate` (delegate `FireInternal`) (`self.FireRate`) true))
        (set `self.FireTimerHandle` _returnvalue)
        (set `/Game/CODE/Player/BP_FPSPlayer.IsFiring` true (`self.Player`))
        (set `self.WeaponState` "NewEnumerator1")
        (else
          (`GameplayStatics.PlaySound2D` "/Game/XL_FPSPack/Weapons/Common/Sounds/Trigger/Dead_trigger/Hand-Guns/Dead_Trigger_Hand-Guns.Dead_Trigger_Hand-Guns" 1.0 1.0 0.0 null null))))))

(event `FireInternal`
  (bind _player (`self.Player`))
  (bind _player_2 (`self.Player`))
  (bind _player_3 (`self.Player`))
  (bind (_returnvalue_location _returnvalue_rotation) (`KismetMathLibrary.BreakTransform` (`SceneComponent.GetSocketTransform` (`self.Weapon`) "Casing" "RTS_World")))
  (bind _camera (`/Game/CODE/Player/BP_FPSPlayer.Camera` (`self.Player`)))
  (bind _returnvalue (`SceneComponent.K2_GetComponentLocation` _camera))
  (bind _returnvalue_2 (`SceneComponent.GetForwardVector` _camera))
  (if (<= (`self.CurrentAmmo`) 0)
    (`self.StopFire`)
    (else
      (`|PlayMontage` (`self.Weapon`) (select `/Game/CODE/Player/System/Enum/E_PlayerState` (`/Game/CODE/Player/BP_FPSPlayer.E_PlayerState` (`self.Player`)) :`NewEnumerator0` (`self.WeaponIdle`) :`NewEnumerator1` (`self.WeaponWalk`) :`NewEnumerator3` (`self.WeaponAim`))
        (:`then`
          (`|PlayMontage` (`/Game/CODE/Player/BP_FPSPlayer.Arm` (`self.Player`)) (select `/Game/CODE/Player/System/Enum/E_PlayerState` (`/Game/CODE/Player/BP_FPSPlayer.E_PlayerState` (`self.Player`)) :`NewEnumerator0` (`self.PlayerIdle`) :`NewEnumerator1` (`self.PlayerWalk`) :`NewEnumerator3` (`self.PlayerAim`))
            (:`then`
              (`GameplayStatics.PlaySound2D` "/Game/CODE/Weapon/MetaSound/MS_Virtus.MS_Virtus" 1.0 1.0 0.0 null null)
              (`NiagaraFunctionLibrary.SpawnSystemAttached` "/Game/ShotSystem/Shot_VFX/VIRTUS_MuzzleFlash.VIRTUS_MuzzleFlash" (`self.Barrel`) "Muzzle" (0.0 0.0 0.0) (struct) "KeepRelativeOffset" true)
              (`/Engine/EditorBlueprintResources/StandardMacros.DecrementInt` (`self.CurrentAmmo`)
                (:`  `
                  (`/Game/CODE/UI/UI_MainUi.UpdateWeaponAmmo` (`/Game/CODE/Player/BP_FPSPlayer.MainUi` (`self.Player`)) (`self.CurrentAmmo`) (`self.TotalAmmo`))
                  (`|SpawnActorFromClass` "/Game/CODE/Weapon/BP_Casing.BP_Casing_C" (`KismetMathLibrary.MakeTransform` _returnvalue_location _returnvalue_rotation) "Undefined" "MultiplyWithRoot" null null)
                  (`Pawn.AddControllerPitchInput` _player -0.4)
                  (`Pawn.AddControllerYawInput` _player (`KismetMathLibrary.RandomFloatInRange` -0.1 0.1))
                  (bind _outhit (`KismetSystemLibrary.LineTraceSingle` _returnvalue (+ _returnvalue (* _returnvalue_2 10000)) "TraceTypeQuery3" false (`|MakeArray` _player_3 (`/Game/CODE/Player/BP_FPSPlayer.CurrentWeapon` _player_3) :!type "Actor Object Reference")))
                  (bind (_bblockinghit _binitialoverlap _time _distance _location _impactpoint _normal _impactnormal _physmat _hitactor) (`GameplayStatics.BreakHitResult` _outhit))
                  (if _bblockinghit
                    (`GameplayStatics.ApplyPointDamage` _hitactor (`self.BaseDamage`) _returnvalue_2 _outhit (`Pawn.GetController` _player_2) (`/Game/CODE/Player/BP_FPSPlayer.CurrentWeapon` _player_2))
                    (`|ExecutionSequence`
                      (:`then_0`
                        (bind _aspawn (cast `Pawn` _hitactor)))
                      (:`then_1`
                        (if (`KismetSystemLibrary.IsValid` _aspawn)
                          (`NiagaraFunctionLibrary.SpawnSystemAtLocation` "/Game/ShotSystem/Shot_VFX/FX_SquibBlood.FX_SquibBlood" _impactpoint (`KismetMathLibrary.MakeRotFromX` _impactnormal) (1.4 1.4 1.4))
                          (else
                            (set `self.Location` _location)
                            (switch `EPhysicalSurface` (`PhysicalMaterial.SurfaceType` _physmat)
                              (:`SurfaceType_Default`
                                (bind _returnvalue_3 (`KismetMathLibrary.MakeRotFromX` _normal))
                                (`NiagaraFunctionLibrary.SpawnSystemAtLocation` "/Game/ShotSystem/Shot_VFX/FX_SquibConcrete.FX_SquibConcrete" (`self.Location`) _returnvalue_3 :!label _label)
                                (`GameplayStatics.PlaySoundAtLocation` "/Game/XL_FPSPack/Common/Sound/Bullet_Impact_Sounds/Concrete/Hit_Concrete.Hit_Concrete" (`self.Location`) (struct) 0.6 1.0 0.0 null null null null)
                                (`|SpawnActorFromClass` "/Game/Decals/BP_BulletDecal.BP_BulletDecal_C" (`KismetMathLibrary.MakeTransform` (`self.Location`) _returnvalue_3 (0.4 0.4 0.4)) "Undefined" "MultiplyWithRoot" null null))
                              (:`SurfaceType1`
                                (`NiagaraFunctionLibrary.SpawnSystemAtLocation` "/Game/ShotSystem/Shot_VFX/FX_SquibDirt.FX_SquibDirt" (`self.Location`) _returnvalue_3)
                                (`GameplayStatics.PlaySoundAtLocation` "/Game/ShotSystem/Shot_SFX/SFX_Vefects_Shots_Squib_Dirt_Cue.SFX_Vefects_Shots_Squib_Dirt_Cue" (`self.Location`) (struct) 1.6 1.0 0.0 null null null null)
                                (bind _returnvalue_4 (`|SpawnActorFromClass` "/Game/Decals/BP_BulletDecal.BP_BulletDecal_C" (`KismetMathLibrary.MakeTransform` (`self.Location`) _returnvalue_3 (0.4 0.4 0.4)) "Undefined" "MultiplyWithRoot" null null))
                                (`DecalComponent.SetDecalMaterial` (`/Game/Decals/BP_BulletDecal.BulletDecal` _returnvalue_4) null))
                              (:`SurfaceType2`
                                (`NiagaraFunctionLibrary.SpawnSystemAtLocation` "/Game/ShotSystem/Shot_VFX/FX_SquibMetal.FX_SquibMetal" (`self.Location`) _returnvalue_3)
                                (`GameplayStatics.PlaySoundAtLocation` "/Game/ShotSystem/Shot_SFX/SFX_Vefects_Shots_Squib_Metal_Cue.SFX_Vefects_Shots_Squib_Metal_Cue" (`self.Location`) (struct) 1.6 1.0 0.0 null null null null)
                                (bind _returnvalue_5 (`|SpawnActorFromClass` "/Game/Decals/BP_BulletDecal.BP_BulletDecal_C" (`KismetMathLibrary.MakeTransform` (`self.Location`) _returnvalue_3 (0.4 0.4 0.4)) "Undefined" "MultiplyWithRoot" null null))
                                (`DecalComponent.SetDecalMaterial` (`/Game/Decals/BP_BulletDecal.BulletDecal` _returnvalue_5) "/Game/Decals/Materials/MI_VFX_BulletDecal_Metal.MI_VFX_BulletDecal_Metal"))
                              (:`SurfaceType3`
                                (`NiagaraFunctionLibrary.SpawnSystemAtLocation` "/Game/ShotSystem/Shot_VFX/FX_SquibWood.FX_SquibWood" (`self.Location`) _returnvalue_3)
                                (`GameplayStatics.PlaySoundAtLocation` "/Game/ShotSystem/Shot_SFX/SFX_Vefects_Shots_Squib_Wood_Cue.SFX_Vefects_Shots_Squib_Wood_Cue" (`self.Location`) (struct) 1.6 1.0 0.0 null null null null)
                                (bind _returnvalue_6 (`|SpawnActorFromClass` "/Game/Decals/BP_BulletDecal.BP_BulletDecal_C" (`KismetMathLibrary.MakeTransform` (`self.Location`) _returnvalue_3 (0.4 0.4 0.4)) "Undefined" "MultiplyWithRoot" null null))
                                (`DecalComponent.SetDecalMaterial` (`/Game/Decals/BP_BulletDecal.BulletDecal` _returnvalue_6) "/Game/Decals/Materials/MI_VFX_BulletDecal_Wood.MI_VFX_BulletDecal_Wood"))
                              (:`SurfaceType4`
                                (`NiagaraFunctionLibrary.SpawnSystemAtLocation` "/Game/XL_FPSPack/Niagara_VFX/Niagara/Impact/Impact_Blood.Impact_Blood" (`self.Location`) _returnvalue_3)
                                (`GameplayStatics.PlaySoundAtLocation` "/Game/XL_FPSPack/Common/Sound/Bullet_Impact_Sounds/Concrete/Hit_Concrete.Hit_Concrete" (`self.Location`) (struct) 1.6 1.0 0.0 null null null null)
                                (`|SpawnActorFromClass` "/Game/Decals/BP_BulletDecal.BP_BulletDecal_C" (`KismetMathLibrary.MakeTransform` (`self.Location`) _returnvalue_3 (0.4 0.4 0.4)) "Undefined" "MultiplyWithRoot" null null))
                              (:`SurfaceType5`
                                (goto _label)))))))))))))))))

(event `StopFire`
  (switch `/Game/CODE/Player/System/Enum/E_WeaponState` (`self.WeaponState`)
    (:`NewEnumerator0`
      _)
    (:`NewEnumerator1`
      _))
  (`KismetSystemLibrary.K2_ClearAndInvalidateTimerHandle` (`self.FireTimerHandle`))
  (set `self.WeaponState` "NewEnumerator0"))

(event `Reload`
  (params (`目标` :type "/Game/CODE/Player/BP_FPSPlayer Object Reference"))
  (set `self.Player` `目标`)
  (switch `/Game/CODE/Player/System/Enum/E_WeaponState` (`self.WeaponState`)
    (:`NewEnumerator0`
      (if (and (< (`self.CurrentAmmo`) (`self.MagSize`)) (> (`self.TotalAmmo`) 0))
        (set `self.WeaponState` "NewEnumerator2")
        (`|PlayMontage` (`self.Weapon`) "/Game/XL_FPSPack/Weapons/MCX-VIRTUS/Animation/Weapon/Weapon_MCX-VIRTUS_Reload_Empty_Montage.Weapon_MCX-VIRTUS_Reload_Empty_Montage"
          (:`then`
            (`|PlayMontage` (`/Game/CODE/Player/BP_FPSPlayer.Arm` (`self.Player`)) "/Game/XL_FPSPack/Weapons/MCX-VIRTUS/Animation/Player/Player_MCX-VIRTUS_Reload_Empty_Montage.Player_MCX-VIRTUS_Reload_Empty_Montage"
              (:`then`
                (`GameplayStatics.PlaySound2D` "/Game/XL_FPSPack/Weapons/MCX-VIRTUS/Sound/Foley/SW_MCX-VIRTUS_Reload_Empty_Foley.SW_MCX-VIRTUS_Reload_Empty_Foley" 1.0 1.0 0.0 null null))
              (:`OnCompleted`
                (set `self.WeaponState` "NewEnumerator0" :!label _label_2))
              (:`OnInterrupted`
                (goto _label_2)))))))))

(fn `GetAimSocketLocation`
  (returns (AimSocketLocation :type "Vector Structure"))
  (bind _output_get (set `self.AimSocketLocation` (`SceneComponent.GetSocketLocation` (`self.Weapon`) "AimSocket")))
  (return _output_get))

(fn `Reload_Ammo`
  (bind _returnvalue (- (`self.MagSize`) (`self.CurrentAmmo`)))
  (if (>= (`self.TotalAmmo`) _returnvalue)
    (set `self.TotalAmmo` (- (`self.TotalAmmo`) _returnvalue))
    (set `self.CurrentAmmo` (`self.MagSize`))
    (else
      (set `self.CurrentAmmo` (+ (`self.CurrentAmmo`) (`self.TotalAmmo`)))
      (set `self.TotalAmmo` 0))))

(fn `UserConstructionScript`)
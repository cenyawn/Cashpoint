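; Actor component that tracks health and death for its owning actor.
; On BeginPlay it binds to the owner's point damage event and routes hits into ApplyDamage, which clamps health and records the last instigator.
; Health changes, damage and death are broadcast through event dispatchers, with a Dead flag blocking further damage or healing until ResetHealth restores full health.
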(event `self.ReceiveBeginPlay`
  (add `Actor.OnTakePointDamage` (`self.GetOwner`) (delegate `OnTakePointDamage_事件`)))

(event `OnTakePointDamage_事件`
  (params (DamagedActor :type "Actor Object Reference") (Damage :type "Float (single-precision)") (InstigatedBy :type "Controller Object Reference") (HitLocation :type "Vector Structure") (FHitComponent :type "PrimitiveComponent Object Reference") (BoneName :type Name) (ShotFromDirection :type "Vector Structure") (DamageType :type "DamageType Object Reference") (DamageCauser :type "Actor Object Reference"))
  (`self.ApplyDamage` Damage InstigatedBy))

(fn `ApplyDamage`
  (params (Damage :type "Float (double-precision)") (Instigator :type "Object Object Reference"))
  (if (not (`self.bDead`))
    (set `self.LastInstigator` Instigator)
    (set `self.Health` (`KismetMathLibrary.FClamp` (- (`self.Health`) Damage) 0.0 (`self.MaxHealth`)))
    (`self.OnHealthChanged` (`self.Health`) (`self.MaxHealth`))
    (`self.OnDamaged` Damage Instigator)
    (if (<= (`self.Health`) 0.0)
      (set `self.bDead` true)
      (`self.OnDeath`))))

(fn `Heal`
  (params (Amount :type "Float (double-precision)"))
  (if (not (`self.bDead`))
    (set `self.Health` (`KismetMathLibrary.FClamp` (+ (`self.Health`) Amount) 0.0 (`self.MaxHealth`)))
    (`self.OnHealthChanged` (`self.Health`) (`self.MaxHealth`))))

(fn `ResetHealth`
  (bind _maxhealth (`self.MaxHealth`))
  (set `self.Health` _maxhealth)
  (set `self.bDead` false)
  (set `self.LastInstigator` null)
  (`self.OnHealthChanged` (`self.Health`) _maxhealth))
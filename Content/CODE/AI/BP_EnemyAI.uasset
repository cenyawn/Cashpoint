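; Enemy AI character that dies into a ragdoll and respawns at its spawn point after a delay.
; On death it rewards the killing player's EconomyComponent once, then stops movement and the controller's StateTree logic.
; A timer calls ForceRespawn, which restores the mesh from transforms cached at BeginPlay, teleports the actor home, resets health and restarts the StateTree.
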(event `self.ReceiveBeginPlay`
  (bind _mesh (`self.Mesh`))
  (set `self.SpawnLocation` (`self.K2_GetActorLocation`))
  (set `self.SpawnRotation` (`self.K2_GetActorRotation`))
  (set `self.MeshRelLocation` (`SceneComponent.RelativeLocation` _mesh))
  (set `self.MeshRelRotation` (`SceneComponent.RelativeRotation` _mesh)))

(event `self.HealthComponent.OnDeath`
  (`self.HandleDeath`))

(event `HandleDeath`
  (bind _mesh (`self.Mesh`))
  (bind _lastinstigator (`/Game/CODE/Combat/BP_HealthComponent.LastInstigator` (`self.HealthComponent`)))
  (`|ExecutionSequence`
    (:`then_0`
      (if (not (`self.bKillRewarded`))
        (set `self.bKillRewarded` true)
        (if (`KismetSystemLibrary.IsValid` _lastinstigator)
          (bind _ascontroller (cast `Controller` _lastinstigator))
          (bind _asbp_fpsplayer (cast `/Game/CODE/Player/BP_FPSPlayer` (`Controller.K2_GetPawn` _ascontroller)))
          (`/Game/CODE/Economy/BP_EconomyComponent.AddKillReward` (`/Game/CODE/Player/BP_FPSPlayer.EconomyComponent` _asbp_fpsplayer)))))
    (:`then_1`
      (`PrimitiveComponent.SetCollisionProfileName` _mesh "Ragdoll" true)
      (`SkeletalMeshComponent.SetAllBodiesSimulatePhysics` _mesh true)
      (bind _asbp_enemy_aicontroller (cast `/Game/CODE/AI/BP_EnemyAIController` (`self.GetController`)))
      (`Controller.StopMovement` _asbp_enemy_aicontroller)
      (`BrainComponent.StopLogic` (`/Game/CODE/AI/BP_EnemyAIController.StateTreeAIComponent` _asbp_enemy_aicontroller) "Death")
      (`CharacterMovementComponent.DisableMovement` (`self.CharacterMovement`))
      (set `self.bCanBeDamaged` false)
      (`KismetSystemLibrary.K2_ClearAndInvalidateTimerHandle` (`self.RespawnTimerHandle`))
      (bind _returnvalue (`KismetSystemLibrary.K2_SetTimerDelegate` (delegate `Respawn`) (`self.RespawnDelay`)))
      (set `self.RespawnTimerHandle` _returnvalue))))

(event `Respawn`
  (`self.ForceRespawn`))

(fn `ForceRespawn`
  (bind _mesh (`self.Mesh`))
  (`KismetSystemLibrary.K2_ClearAndInvalidateTimerHandle` (`self.RespawnTimerHandle`))
  (`SkeletalMeshComponent.SetAllBodiesSimulatePhysics` _mesh false)
  (`PrimitiveComponent.SetCollisionProfileName` _mesh "CharacterMesh" true)
  (`SceneComponent.K2_SetRelativeLocationAndRotation` _mesh (`self.MeshRelLocation`) (`self.MeshRelRotation`) false false)
  (`self.K2_SetActorLocationAndRotation` (`self.SpawnLocation`) (`self.SpawnRotation`) false true)
  (`self.SetActorHiddenInGame` false)
  (`self.SetActorEnableCollision` true)
  (`CharacterMovementComponent.SetMovementMode` (`self.CharacterMovement`) "MOVE_Walking" 0)
  (`/Game/CODE/Combat/BP_HealthComponent.ResetHealth` (`self.HealthComponent`))
  (set `self.bCanBeDamaged` true)
  (set `self.bKillRewarded` false)
  (bind _asbp_enemy_aicontroller (cast `/Game/CODE/AI/BP_EnemyAIController` (`self.GetController`)))
  (`BrainComponent.StartLogic` (`/Game/CODE/AI/BP_EnemyAIController.StateTreeAIComponent` _asbp_enemy_aicontroller)))

(fn `UserConstructionScript`)
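; BP_Merchant is a team-colored merchant that lets the local player open or close a shop with an interact press.
; Tick polls the cached BP_FPSPlayer for radius, height, alive, no open UI and optional same-team checks, calling ToggleMerchantShop on the press edge.
; The resulting in-range flag drives a team-labeled widget prompt, updated only on visibility changes.
; A looping timer yaws the visible prompt toward the camera.
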(event `self.ReceiveBeginPlay`
  (`KismetSystemLibrary.K2_SetTimerDelegate` (delegate `OnFacePromptTimer`) 0.1 true)
  (`self.InitMerchant`))

(event `self.ReceiveTick`
  (params (DeltaSeconds :type "Float (single-precision)"))
  (`self.UpdateInteraction`))

(event `OnFacePromptTimer`
  (if (`self.bPlayerInRange`)
    (`self.FacePromptToCamera`)))

(fn `FacePromptToCamera`
  (bind _promptcomp (`self.PromptComp`))
  (`SceneComponent.K2_SetWorldRotation` _promptcomp (`KismetMathLibrary.MakeRotator` 0.0 0.0 (.yaw (`KismetMathLibrary.FindLookAtRotation` (`SceneComponent.K2_GetComponentLocation` _promptcomp) (`PlayerCameraManager.GetCameraLocation` (`GameplayStatics.GetPlayerCameraManager` 0))))) false false))

(fn `InitMerchant`
  (bind _asui_merchant_prompt (cast `/Game/CODE/UI/UI_MerchantPrompt` (`WidgetComponent.GetUserWidgetObject` (`self.PromptComp`))))
  (set `self.PromptWidget` _asui_merchant_prompt)
  (`self.SetTeamColor`)
  (`self.RefreshPrompt`))

(fn `RefreshPrompt`
  (bind _promptcomp (`self.PromptComp`))
  (bind _bplayerinrange (`self.bPlayerInRange`))
  (bind _promptwidget (`self.PromptWidget`))
  (if (`KismetSystemLibrary.IsValid` _promptwidget)
    (if (xor _bplayerinrange (`self.LastPromptVisible`))
      (if (== (`self.TeamId`) 0) :!label _label
        (`/Game/CODE/UI/UI_MerchantPrompt.SetNameText` _promptwidget "RED MERCHANT")
        (`/Game/CODE/UI/UI_MerchantPrompt.SetNameColor` _promptwidget (struct :`R` 1.0 :`G` 0.1 :`B` 0.06 :`A` 1.0))
        (else
          (`/Game/CODE/UI/UI_MerchantPrompt.SetNameText` _promptwidget "BLUE MERCHANT")
          (`/Game/CODE/UI/UI_MerchantPrompt.SetNameColor` _promptwidget (struct :`R` 0.1 :`G` 0.35 :`B` 1.0 :`A` 1.0))))
      (`/Game/CODE/UI/UI_MerchantPrompt.SetPrompt` _promptwidget _bplayerinrange "Press F to trade")
      (`SceneComponent.SetVisibility` _promptcomp _bplayerinrange false)
      (set `self.LastPromptVisible` _bplayerinrange))
    (else
      (bind _asui_merchant_prompt (cast `/Game/CODE/UI/UI_MerchantPrompt` (`WidgetComponent.GetUserWidgetObject` _promptcomp)))
      (set `self.PromptWidget` _asui_merchant_prompt)
      (goto _label))))

(fn `SetTeamColor`
  (bind _mesh (`self.Mesh`))
  (if (== (`self.TeamId`) 0)
    (`PrimitiveComponent.SetMaterial` _mesh 0 "/Game/CODE/Merchant/Materials/MI_Merchant_Red.MI_Merchant_Red")
    (`PrimitiveComponent.SetMaterial` _mesh 1 "/Game/CODE/Merchant/Materials/MI_Merchant_Red.MI_Merchant_Red")
    (else
      (`PrimitiveComponent.SetMaterial` _mesh 0 "/Game/CODE/Merchant/Materials/MI_Merchant_Blue.MI_Merchant_Blue")
      (`PrimitiveComponent.SetMaterial` _mesh 1 "/Game/CODE/Merchant/Materials/MI_Merchant_Blue.MI_Merchant_Blue"))))

(fn `UpdateInteraction`
  (bind _returnvalue (`self.K2_GetActorLocation`))
  (bind _playerref (`self.PlayerRef`))
  (bind _returnvalue_2 (`self.K2_GetActorLocation` _playerref))
  (bind _returnvalue_3 (`KismetSystemLibrary.IsValid` _playerref))
  (bind _binteractheld (`/Game/CODE/Player/BP_FPSPlayer.bInteractHeld` _playerref))
  (bind _healthcomponent (`/Game/CODE/Player/BP_FPSPlayer.HealthComponent` _playerref))
  (bind _returnvalue_4 (and (and (and (and (<= (`KismetMathLibrary.Vector_Distance2D` _returnvalue_2 _returnvalue) (`self.InteractRadius`)) (<= (`KismetMathLibrary.Abs` (- (.z _returnvalue_2) (.z _returnvalue))) (`self.InteractZRange`))) (not (`/Game/CODE/Combat/BP_HealthComponent.bDead` _healthcomponent))) (not (`/Game/CODE/Player/BP_FPSPlayer.bUIOpen` _playerref))) (or (not (`self.bRestrictToOwnTeam`)) (== (`/Game/CODE/Combat/BP_HealthComponent.TeamId` _healthcomponent) (`self.TeamId`)))))
  (if _returnvalue_3
    (if _returnvalue_3 :!label _label
      (if (and _returnvalue_4 (and _binteractheld (not (`self.bInteractPrev`))))
        (`/Game/CODE/Player/BP_FPSPlayer.ToggleMerchantShop` _playerref))
      (set `self.bPlayerInRange` _returnvalue_4)
      (set `self.bInteractPrev` _binteractheld)
      (else
        (set `self.bPlayerInRange` false :!label _label_2)
        (set `self.bInteractPrev` false)))
    (else
      (bind _asbp_fpsplayer (cast `/Game/CODE/Player/BP_FPSPlayer` (`GameplayStatics.GetPlayerCharacter` 0))
        (:`then`
          (set `self.PlayerRef` _asbp_fpsplayer)
          (goto _label))
        (:`CastFailed`
          (goto _label_2)))))
  (`self.RefreshPrompt`))

(fn `UserConstructionScript`)
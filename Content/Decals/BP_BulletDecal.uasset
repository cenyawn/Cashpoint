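; Bullet impact decal actor that leaves a varied mark where a shot lands.
; On BeginPlay it gives the BulletDecal component a random roll and random Y/Z scale so repeated hits look different.
; ConfigureDecal lets a caller set the material, scale and lifespan, with its scale replacing the current one.
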(event `self.ReceiveBeginPlay`
  (bind _returnvalue (`KismetMathLibrary.RandomFloatInRange` 0.29 0.45))
  (bind _bulletdecal (`self.BulletDecal`))
  (`SceneComponent.K2_AddRelativeRotation` _bulletdecal (`KismetMathLibrary.MakeRotator` (`KismetMathLibrary.RandomFloatInRange` 0.0 360.0)) false false)
  (`SceneComponent.SetRelativeScale3D` _bulletdecal (`KismetMathLibrary.MakeVector` 1.0 _returnvalue _returnvalue)))

(fn `ConfigureDecal`
  (params (Material :type "MaterialInterface Object Reference") (Size :type "Vector Structure") (LifeSeconds :type "Float (double-precision)"))
  (bind _bulletdecal (`self.BulletDecal`))
  (`DecalComponent.SetDecalMaterial` _bulletdecal Material)
  (`SceneComponent.SetRelativeScale3D` _bulletdecal Size)
  (`self.SetLifeSpan` self LifeSeconds))

(fn `UserConstructionScript`)